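; Elevator actor that raises and lowers a Lift between a start position and a Destination component, carrying the VR motion controller pawn.
; ToggleElevator flips the direction and calls MoveElevator, which plays or reverses a timeline that lerps the Lift's relative location.
; A collider attaches the overlapping pawn to the Lift and detaches it on exit.
; Logic to snap the pawn's height exists but is unconnected.
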(event `self.ReceiveBeginPlay`
  (set `self.ElevatorEnd` (`SceneComponent.RelativeLocation` (`self.Destination`))))

(event `MoveElevator`
  (params (bIsUp :type Boolean))
  (if bIsUp
    (bind (_direction _height_lerp) (`Timeline|ListDriver` :!label _label)
      (:`Update`
        (`SceneComponent.K2_SetRelativeLocation` (`self.Lift`) (`KismetMathLibrary.VLerp` (`self.ElevatorStart`) (`self.ElevatorEnd`) _height_lerp) false false)))
    (else
      (goto _label :!via `Reverse`))))

(event `ToggleElevator`
  (bind _output_get (set `self.bIsUp` (not (`self.bIsUp`))))
  (`self.MoveElevator` _output_get))

(event `self.Player_Collider.OnComponentBeginOverlap`
  (params (OverlappedComponent :type "PrimitiveComponent Object Reference") (OtherActor :type "Actor Object Reference") (OtherComp :type "PrimitiveComponent Object Reference") (OtherBodyIndex :type Integer) (bFromSweep :type Boolean) (SweepResult :type "HitResult Structure (by ref)"))
  (bind _asmotion_controller_pawn (cast `/Game/VirtualRealityBP/Blueprints/MotionControllerPawn` OtherActor))
  (bind _output_get (set `self.PlayerPawn` _asmotion_controller_pawn))
  (`self.K2_AttachToComponent` _output_get (`self.Lift`) "None" "KeepWorld" "KeepWorld" "KeepWorld" false))

(event `self.Player_Collider.OnComponentEndOverlap`
  (params (OverlappedComponent :type "PrimitiveComponent Object Reference") (OtherActor :type "Actor Object Reference") (OtherComp :type "PrimitiveComponent Object Reference") (OtherBodyIndex :type Integer))
  (bind _playerpawn (`self.PlayerPawn`))
  (bind _asmotion_controller_pawn (cast `/Game/VirtualRealityBP/Blueprints/MotionControllerPawn` OtherActor))
  (`/Engine/EditorBlueprintResources/StandardMacros.IsValid` _playerpawn
    (:`Is Valid`
      (if (== _asmotion_controller_pawn _playerpawn)
        (`self.K2_DetachFromActor` (`self.PlayerPawn`) "KeepWorld" "KeepWorld" "KeepWorld")
        (set `self.PlayerPawn` null)))))

(fn `UserConstructionScript`)