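; WorldInteractive is an interface-style Blueprint defining how world objects respond to an interactor.
; It declares callbacks for hover, use and pickup press/release, dragging, and hovered-component changes, each taking the Interactor and returning a boolean.
; GetClosestComponentData returns a point and priority for a given interactor.
; All functions here are stubs returning false or zero defaults, with no logic of their own.
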(fn `GetClosestComponentData`
  (params (Interactor :type "/Game/Meshes/ExampleContent/VR_World_Interaction/Blueprints/Components/BPC_WorldInteractor Object Reference"))
  (returns (Point :type "Vector Structure") (Priority :type Integer) (Component :type "SceneComponent Object Reference"))
  (return (0.0 0.0 0.0) 0 null))

(fn `OnDrag`
  (params (Interactor :type "/Game/Meshes/ExampleContent/VR_World_Interaction/Blueprints/Components/BPC_WorldInteractor Object Reference"))
  (returns (Return :type Boolean))
  (return false))

(fn `OnDragStart`
  (params (Interactor :type "/Game/Meshes/ExampleContent/VR_World_Interaction/Blueprints/Components/BPC_WorldInteractor Object Reference"))
  (returns (Return :type Boolean))
  (return false))

(fn `OnDragStop`
  (params (Interactor :type "/Game/Meshes/ExampleContent/VR_World_Interaction/Blueprints/Components/BPC_WorldInteractor Object Reference"))
  (returns (Return :type Boolean))
  (return false))

(fn `OnHover`
  (params (Interactor :type "/Game/Meshes/ExampleContent/VR_World_Interaction/Blueprints/Components/BPC_WorldInteractor Object Reference"))
  (returns (Return :type Boolean))
  (return false))

(fn `OnHoveredComponentChanged`
  (params (Interactor :type "/Game/Meshes/ExampleContent/VR_World_Interaction/Blueprints/Components/BPC_WorldInteractor Object Reference") (OldComponent :type "SceneComponent Object Reference") (NewComponent :type "SceneComponent Object Reference"))
  (returns (Return :type Boolean))
  (return false))

(fn `OnPickupPressed`
  (params (Interactor :type "/Game/Meshes/ExampleContent/VR_World_Interaction/Blueprints/Components/BPC_WorldInteractor Object Reference"))
  (returns (Return :type Boolean))
  (return false))

(fn `OnPickupReleased`
  (params (Interactor :type "/Game/Meshes/ExampleContent/VR_World_Interaction/Blueprints/Components/BPC_WorldInteractor Object Reference"))
  (returns (Return :type Boolean))
  (return false))

(fn `OnUnHover`
  (params (Interactor :type "/Game/Meshes/ExampleContent/VR_World_Interaction/Blueprints/Components/BPC_WorldInteractor Object Reference"))
  (returns (Return :type Boolean))
  (return false))

(fn `OnUsePressed`
  (params (Interactor :type "/Game/Meshes/ExampleContent/VR_World_Interaction/Blueprints/Components/BPC_WorldInteractor Object Reference"))
  (returns (Return :type Boolean))
  (return false))

(fn `OnUseReleased`
  (params (Interactor :type "/Game/Meshes/ExampleContent/VR_World_Interaction/Blueprints/Components/BPC_WorldInteractor Object Reference"))
  (returns (Return :type Boolean))
  (return false))