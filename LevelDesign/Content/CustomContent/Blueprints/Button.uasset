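; A pressable VR button that toggles a linked sliding door or elevator.
; A motion controller overlapping its box triggers PressButton, which is locked out until a timeline finishes moving the cylinder between start and end positions.
; The press casts the assigned DoorActor to SlidingDoor, then Elevator, to call its toggle, printing a warning when none is connected.
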(event `PressButton`
  (bind _dooractor (`self.DoorActor`))
  (if (`self.bCanPress`)
    (`|ExecutionSequence`
      (:`then_0`
        (set `self.bCanPress` false)
        (bind (_direction _button_position_float) (`Timeline|ButtonDriver` :!via `PlayFromStart`)
          (:`Update`
            (`SceneComponent.K2_SetRelativeLocation` (`self.Cylinder`) (`KismetMathLibrary.VLerp` (`self.StartLoc`) (`self.EndLoc`) _button_position_float) false false))
          (:`Finished`
            (set `self.bCanPress` true))))
      (:`then_1`
        (`/Engine/EditorBlueprintResources/StandardMacros.IsValid` _dooractor
          (:`Is Valid`
            (bind _assliding_door (cast `/Game/CustomContent/Blueprints/SlidingDoor` _dooractor)
              (:`then`
                (`/Game/CustomContent/Blueprints/SlidingDoor.ToggleDoor` _assliding_door))
              (:`CastFailed`
                (bind _aselevator (cast `/Game/CustomContent/Blueprints/Elevator` _dooractor))
                (`/Game/CustomContent/Blueprints/Elevator.ToggleElevator` _aselevator))))
          (:`Is Not Valid`
            (`KismetSystemLibrary.PrintString` "No door connected to button")))))))

(event `self.Box.OnComponentBeginOverlap`
  (params (OverlappedComponent :type "PrimitiveComponent Object Reference") (OtherActor :type "Actor Object Reference") (OtherComp :type "PrimitiveComponent Object Reference") (OtherBodyIndex :type Integer) (bFromSweep :type Boolean) (SweepResult :type "HitResult Structure (by ref)"))
  (cast `/Game/VirtualRealityBP/Blueprints/BP_MotionController` OtherActor)
  (`self.PressButton`))

(event `self.Box.OnComponentEndOverlap`
  (params (OverlappedComponent :type "PrimitiveComponent Object Reference") (OtherActor :type "Actor Object Reference") (OtherComp :type "PrimitiveComponent Object Reference") (OtherBodyIndex :type Integer))
  (cast `/Game/VirtualRealityBP/Blueprints/BP_MotionController` OtherActor))

(fn `UserConstructionScript`)