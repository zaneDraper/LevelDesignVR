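; VR gun actor that can be picked up, dropped and fired at destructible objects and buttons.
; Pickup attaches it to the given component with grip offsets for Oculus Rift or Steam VR; Drop detaches it in place with physics off.
; Firing line-traces along the gun's negative right vector, plays hand haptics and an explosion, then applies radius damage to destructibles or presses Buttons.
; A separate rumble event sends brief left-side force feedback.
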(event `EventFire`
  (params (GunHand :type "EControllerHand Enum"))
  (bind _gun (`self.Gun`))
  (bind _returnvalue (`SceneComponent.K2_GetComponentLocation` _gun))
  (bind _outhit (`KismetSystemLibrary.LineTraceSingle` _returnvalue (+ (* (`SceneComponent.GetRightVector` _gun) -3000.0) _returnvalue) "TraceTypeQuery1"))
  (`self.HandleTargetHit` _outhit GunHand))

(event `/Game/VirtualRealityBP/Blueprints/PickupActorInterface.Drop`
  (`PrimitiveComponent.SetSimulatePhysics` (`self.Gun`) false)
  (`self.K2_DetachFromActor` "KeepWorld" "KeepWorld" "KeepWorld"))

(event `/Game/VirtualRealityBP/Blueprints/PickupActorInterface.Pickup`
  (params (AttachTo :type "SceneComponent Object Reference"))
  (bind _gun (`self.Gun`))
  (bind _gun_2 (`self.Gun`))
  (`PrimitiveComponent.SetSimulatePhysics` (`self.Gun`) false)
  (`SceneComponent.K2_AttachToComponent` (`self.K2_GetRootComponent`) AttachTo "None" "SnapToTarget" "SnapToTarget" "KeepWorld" false)
  (switch `name` (`HeadMountedDisplayFunctionLibrary.GetHMDDeviceName`)
    (:`OculusRift`
      (`SceneComponent.K2_AddRelativeLocation` _gun (3.5 -1.0 0.5) false false)
      (`SceneComponent.K2_AddRelativeRotation` _gun (struct :`Yaw` 90.0) false false))
    (:`SteamVR`
      (`SceneComponent.K2_AddRelativeLocation` _gun_2 (7.0 0.0 -9.0) false false)
      (`SceneComponent.K2_AddRelativeRotation` _gun_2 (struct :`Yaw` 90.0 :`Roll` -45.0) false false))))

(event `RumbleController`
  (params (Intensity :type "Float (double-precision)"))
  (bind _returnvalue (select `EControllerHand` "Left" :`Left` true))
  (bind _returnvalue_2 (not _returnvalue))
  (`PlayerController.PlayDynamicForceFeedback` (`GameplayStatics.GetPlayerController` 0) Intensity 0.07 _returnvalue _returnvalue _returnvalue_2 _returnvalue_2))

(event `HandleTargetHit`
  (params (Hit :type "HitResult Structure") (Hand :type "EControllerHand Enum"))
  (bind (_bblockinghit _binitialoverlap _time _location _impactpoint _normal _impactnormal _physmat _hitactor _hitcomponent) (`GameplayStatics.BreakHitResult` Hit))
  (`PlayerController.PlayHapticEffect` (`GameplayStatics.GetPlayerController` 0) "/Game/CustomContent/Others/GunShot_Feedback.GunShot_Feedback" Hand 0.5 false)
  (bind _returnvalue (`GameplayStatics.SpawnEmitterAtLocation` "/Game/StarterContent/Particles/P_Explosion.P_Explosion" _location))
  (`SceneComponent.SetRelativeScale3D` _returnvalue (0.5 0.5 0.5))
  (`KismetSystemLibrary.PrintString` (`KismetSystemLibrary.GetObjectName` _hitcomponent))
  (bind _asdestructible_actor (cast `DestructibleActor` _hitactor)
    (:`then`
      (`DestructibleComponent.ApplyRadiusDamage` (`DestructibleActor.DestructibleComponent` _asdestructible_actor) 15.0 _location 30.0 10000.0 false))
    (:`CastFailed`
      (bind _asbutton (cast `/Game/CustomContent/Blueprints/Button` _hitactor))
      (`/Game/CustomContent/Blueprints/Button.PressButton` _asbutton))))

(fn `UserConstructionScript`)