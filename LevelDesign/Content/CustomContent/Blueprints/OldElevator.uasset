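; OldElevator is an elevator actor that equips itself with an interactive lever at runtime.
; On BeginPlay it spawns a BP_InteractiveLever at the LeverSpawn transform, scaled down, and attaches it to the Lift component keeping world transform.
; It then passes itself to the lever as its Elevator reference; the graphs shown contain no movement logic.
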(event `self.ReceiveBeginPlay`
  (bind (_returnvalue_location _returnvalue_rotation _returnvalue_scale) (`KismetMathLibrary.BreakTransform` (`SceneComponent.K2_GetComponentToWorld` (`self.LeverSpawn`))))
  (`parent.ReceiveBeginPlay`)
  (bind _returnvalue (`|SpawnActorFromClass` "/Game/Meshes/ExampleContent/VR_World_Interaction/Blueprints/InteractiveObjects/BP_InteractiveLever.BP_InteractiveLever_C" (`KismetMathLibrary.MakeTransform` _returnvalue_location _returnvalue_rotation (/ _returnvalue_scale 2.5)) "Undefined" "OverrideRootScale"))
  (`self.K2_AttachToComponent` _returnvalue (`self.Lift`) "None" "KeepWorld" "KeepWorld" "KeepWorld" true)
  (set `/Game/Meshes/ExampleContent/VR_World_Interaction/Blueprints/InteractiveObjects/BP_InteractiveLever.Elevator` self _returnvalue))

(fn `UserConstructionScript`
  (`parent.UserConstructionScript`))