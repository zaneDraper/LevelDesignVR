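; Sliding door Blueprint that moves its Door component between an open and a closed position.
; ToggleDoor flips the DoorOpen flag and passes it to the OpenCloseDoor event, which plays or reverses the DoorDriver timeline.
; The timeline's output drives a lerp from DoorStart to DoorEnd that sets the door's relative location without sweep.
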(event `OpenCloseDoor`
  (params (bOpenDoor :type Boolean))
  (if bOpenDoor
    (bind (_direction _driver) (`Timeline|DoorDriver` :!label _label)
      (:`Update`
        (`SceneComponent.K2_SetRelativeLocation` (`self.Door`) (`KismetMathLibrary.VLerp` (`self.DoorStart`) (`self.DoorEnd`) _driver) false false)))
    (else
      (goto _label :!via `Reverse`))))

(fn `ToggleDoor`
  (bind _output_get (set `self.bDoorOpen` (not (`self.bDoorOpen`))))
  (`self.OpenCloseDoor` _output_get))

(fn `UserConstructionScript`)