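; KeyDoor is a door that unlocks and swings open when the correct Key_Pickup enters its trigger box.
; A right key hides its pickup mesh, reveals AnimKey, and after a short delay calls OpenDoor.
; OpenDoor plays the KeyDriver timeline, whose separate tracks lerp the key's position and rotation and the door Scene's rotation.
; A wrong key shows WrongKeyIndicator, which hides when a key leaves the box.
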(event `self.ReceiveBeginPlay`)

(event `OpenDoor`
  (bind _animkey (`self.AnimKey`))
  (bind (_direction _keyposdriver _keyrotdriver _doordriver) (`Timeline|KeyDriver` :!via `PlayFromStart`)
    (:`Update`
      (`SceneComponent.K2_SetRelativeRotation` _animkey (`KismetMathLibrary.RLerp` (`self.KeyStartRot`) (`self.KeyEndRot`) _keyrotdriver) false false)
      (`SceneComponent.K2_SetRelativeLocation` _animkey (`KismetMathLibrary.VLerp` (`self.KeyStartLoc`) (`self.KeyEndLoc`) _keyposdriver) false false)
      (`SceneComponent.K2_SetRelativeRotation` (`self.Scene`) (`KismetMathLibrary.RLerp` (`self.DoorStartRotation`) (`self.DoorEndRotation`) _doordriver true) false false))))

(event `self.Box.OnComponentBeginOverlap`
  (params (OverlappedComponent :type "PrimitiveComponent Object Reference") (OtherActor :type "Actor Object Reference") (OtherComp :type "PrimitiveComponent Object Reference") (OtherBodyIndex :type Integer) (bFromSweep :type Boolean) (SweepResult :type "HitResult Structure (by ref)"))
  (bind _askey_pickup (cast `/Game/CustomContent/Blueprints/PickupObjects/Key_Pickup` OtherActor))
  (if (`/Game/CustomContent/Blueprints/PickupObjects/Key_Pickup.bIsRightKey` _askey_pickup)
    (`SceneComponent.SetVisibility` (`StaticMeshActor.StaticMeshComponent` _askey_pickup) false true)
    (`SceneComponent.SetVisibility` (`self.AnimKey`) true true)
    (`KismetSystemLibrary.Delay` 0.1)
    (`self.OpenDoor`)
    (else
      (`SceneComponent.SetVisibility` (`self.WrongKey_Indicator`) true true))))

(event `self.Box.OnComponentEndOverlap`
  (params (OverlappedComponent :type "PrimitiveComponent Object Reference") (OtherActor :type "Actor Object Reference") (OtherComp :type "PrimitiveComponent Object Reference") (OtherBodyIndex :type Integer))
  (cast `/Game/CustomContent/Blueprints/PickupObjects/Key_Pickup` OtherActor)
  (`SceneComponent.SetVisibility` (`self.WrongKey_Indicator`) false false))

(fn `UserConstructionScript`)